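; Spike bomb Blueprint that handles defuse and detonation feedback, with a lethal expanding blast zone.
; Detonation enables query collision on InnerMesh and runs the Bomb timeline to scale DeadZone.
; An agent overlapping InnerMesh has its locally controlled client ask the server to apply the GE_Dead gameplay effect.
; Defuse start plays a 2D sound, the planting handler is empty, and the countdown audio chain is disconnected.
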(event `self.HandlePlantingStarted`)

(event `self.HandleDefusingStarted`
  (`GameplayStatics.PlaySound2D` "/Game/Resource/Audio/Spike/스파이크_해체_누르기_.스파이크_해체_누르기_" 1.0 1.0 0.0 null null))

(event `self.HandleDetonated`
  (`PrimitiveComponent.SetCollisionEnabled` (`self.InnerMesh`) "QueryOnly")
  (bind (_direction _deadzonescale) (`Timeline|Bomb`)
    (:`Update`
      (`SceneComponent.SetWorldScale3D` (`self.DeadZone`) (`KismetMathLibrary.Conv_DoubleToVector` _deadzonescale)))))

(event `BombTest`
  (`self.HandleDetonated`))

(event `self.InnerMesh.OnComponentBeginOverlap`
  (params (OverlappedComponent :type "PrimitiveComponent Object Reference") (OtherActor :type "Actor Object Reference") (OtherComp :type "PrimitiveComponent Object Reference") (OtherBodyIndex :type Integer) (bFromSweep :type Boolean) (SweepResult :type "HitResult Structure (by ref)"))
  (bind _asbase_agent (cast `BaseAgent` OtherActor))
  (if (`Pawn.IsLocallyControlled` _asbase_agent)
    (`BaseAgent.ServerApplyGE` _asbase_agent "/Game/BluePrint/GAS/Effects/GE_Dead.GE_Dead_C" null)))

(fn `UserConstructionScript`)